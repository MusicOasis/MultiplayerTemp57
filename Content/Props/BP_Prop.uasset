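; BP_Prop is a template interactable prop with flag-selected proximity, prompted proximity, cursor-click and cursor-hover interactions.
; TriggerBox overlaps by the player either fire the no-prompt events or toggle the WBP_Interact prompt and AllowInteraction.
; In prompt mode, BeginPlay binds to BP_ThirdPersonCharacter's interact event, which runs PromptInteraction while allowed.
; Interaction responses are placeholder prints, except no-prompt entry, which also plays WaveFile through WavePlayer.
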(event OnComponentEndOverlap(TriggerBox)
  (params (OverlappedComponent :type Primitive%20Component%20Object%20Reference) (OtherActor :type Actor%20Object%20Reference) (OtherComp :type Primitive%20Component%20Object%20Reference) (OtherBodyIndex :type Integer))
  (bind _returnvalue (Game|GetPlayerCharacter 0))
  ;[0.15 0.15 0.15 0.5] Proximity Based Select with Prompt
  (if (Variables|Default|GetUseProximityInteractionNoPrompt)
    (if (== _returnvalue OtherActor)
      (CallFunction|NoPromptInteractionCollisionEnd))
    (elif (Variables|Default|GetUseProximityInteractionWithPrompt)
      (if (== _returnvalue OtherActor)
        (Widget|RemovefromParent (Variables|Default|GetInteractPrompt))
        (Variables|Default|SetAllowInteraction false)))))

(event OnBeginCursorOver(Object)
  (params (TouchedComponent :type Primitive%20Component%20Object%20Reference))
  ;[0.15 0.15 0.15 0.5] Action to Take after Interaction
  (if (Variables|Default|GetUseCursorHoverInteraction)
    (Development|PrintString "Execute Unique On Hover Interaction Code")))

(event OnEndCursorOver(Object)
  (params (TouchedComponent :type Primitive%20Component%20Object%20Reference))
  ;[0.15 0.15 0.15 0.5] Action to Take after Interaction
  (if (Variables|Default|GetUseCursorHoverInteraction)
    (Development|PrintString "Execute Unique On Hover End Interaction Code")))

(event OnClicked(Object)
  (params (TouchedComponent :type Primitive%20Component%20Object%20Reference) (ButtonPressed :type Key%20Structure :default "None"))
  ;[0.15 0.15 0.15 0.5] Action to Take after Interaction
  (if (Variables|Default|GetUseCursorSelectInteraction)
    (if (== ButtonPressed "LeftMouseButton")
      (Development|PrintString "Execute Unique On Click Interaction Code"))))

(event OnComponentBeginOverlap(TriggerBox)
  (params (OverlappedComponent :type Primitive%20Component%20Object%20Reference) (OtherActor :type Actor%20Object%20Reference) (OtherComp :type Primitive%20Component%20Object%20Reference) (OtherBodyIndex :type Integer) (bFromSweep :type Boolean) (SweepResult :type Hit%20Result%20Structure%20%28by%20ref%29))
  (bind _returnvalue (Game|GetPlayerCharacter 0))
  ;[0.15 0.15 0.15 0.5] Proximity Based Select with Prompt
  (if (Variables|Default|GetUseProximityInteractionNoPrompt)
    (if (== OtherActor _returnvalue)
      (CallFunction|NoPromptCollsionInteraction))
    (elif (Variables|Default|GetUseProximityInteractionWithPrompt)
      (if (== OtherActor _returnvalue)
        (UserInterface|Viewport|AddtoViewport (Variables|Default|GetInteractPrompt) 0)
        (Variables|Default|SetAllowInteraction true)))))

(event Custom|NoPromptInteractionCollisionEnd
  ;[0.15 0.15 0.15 0.5] Action to Take after Interaction
  (Development|PrintString "Execute Unique Proximity No Prompt Interaction End Code"))

(event Custom|InteractEventTriggered
  ;[0.15 0.15 0.15 0.5] Setup Proximity Select
  (if (Variables|Default|GetAllowInteraction)
    (CallFunction|PromptInteraction)))

(event Custom|PromptInteraction
  ;[0.15 0.15 0.15 0.5] Action to Take after Interaction
  (Widget|RemovefromParent (Variables|Default|GetInteractPrompt))
  (Variables|Default|SetAllowInteraction true)
  (Development|PrintString "Execute Unique Proximity Interaction Code"))

(event Custom|NoPromptCollsionInteraction
  ;[0.15 0.15 0.15 0.5] Action to Take after Interaction
  (Development|PrintString "Execute Unique Proximity No Prompt Interaction Code")
  (Audio|Components|Audio|SetSound (Variables|Default|GetWavePlayer) (Variables|Default|GetWaveFile))
  (Audio|Components|Audio|Play (Variables|Default|GetWavePlayer) 0.0))

(event EventBeginPlay
  ;[0.15 0.15 0.15 0.5] Setup Proximity Select
  (if (Variables|Default|GetUseProximityInteractionWithPrompt)
    (bind _returnvalue (Game|ConstructObjectfromClass "/Game/UI/WBP_Interact.WBP_Interact_C"))
    (Variables|Default|SetInteractPrompt _returnvalue)
    (bind _asbp_third_person_character (Utilities|Casting|CastToBP_ThirdPersonCharacter (Game|GetPlayerCharacter 0)))
    (EventDispatchers|BindEventtoInteractProximityEventTriggered _asbp_third_person_character (delegate Custom|InteractEventTriggered))))

(fn ConstructionScript)